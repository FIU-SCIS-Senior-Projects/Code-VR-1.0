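; GameController is a Blueprint that moves the first actor in its Cubes array toward the first Destinations actor while a flag is set.
; Each Tick it eases linearly from the cube's current location, with alpha built from DeltaSeconds times one variable plus another.
; The alpha restarts from the current position rather than accumulating, and the value stored afterward is not read back in this graph.
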(event `self.ReceiveBeginPlay`)

(event `self.ReceiveTick`
  (params (DeltaSeconds :type "Float (single-precision)"))
  (bind _output (`|GetArrayItem` (`self.Cubes`)))
  (bind _returnvalue (+ (* DeltaSeconds (`self.NewVar_1`)) (`self.NewVar_2`)))
  (if (`self.NewVar_0`)
    (`self.K2_SetActorLocation` _output (`|EaseFunction` "Linear" _returnvalue (`self.K2_GetActorLocation` _output) (`self.K2_GetActorLocation` (`|GetArrayItem` (`self.Destinations`)))) false false)
    (set `self.NewVar_3` _returnvalue)))

(fn `UserConstructionScript`)